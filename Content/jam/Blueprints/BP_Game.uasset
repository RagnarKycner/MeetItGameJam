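; BP_Game is a game-state Blueprint for a jam game that tracks elapsed play time and handles the death condition.
; Tick drives a one-second Delay as a makeshift clock, incrementing Seconds and rolling over into Minutes after 59.
; In parallel, Tick polls Lifes and, at zero, adds the Dead widget to the viewport and pauses the game.
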(event `self.ReceiveTick`
  (params (DeltaSeconds :type "Float (single-precision)"))
  (`|ExecutionSequence`
    (:`then_0`
      (`KismetSystemLibrary.Delay` 1.0)
      (if (== (`self.seconds`) 59)
        (set `self.minutes` (+ (`self.minutes`) 1))
        (set `self.seconds` 0)
        (else
          (set `self.seconds` (+ (`self.seconds`) 1)))))
    (:`then_1`
      (if (== (`self.Lifes`) 0)
        (bind _returnvalue (`|CreateWidget` "/Game/jam/widget/dead.dead_C"))
        (`UserWidget.AddToViewport` _returnvalue 0)
        (`GameplayStatics.SetGamePaused` true)))))

(fn `UserConstructionScript`)